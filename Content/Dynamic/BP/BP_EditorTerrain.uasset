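; Editor terrain actor that shows an assigned mesh and exposes events to create or clear a river spline.
; The construction script applies Mesh to GeneratedStaticMesh.
; CreateRiver caches local spline points and clears the spline, but its re-add loop reads the cleared count, then it nudges the actor and leaves it at world origin.
; ClearRiverSpline removes all spline points.
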(event Custom|CreateRiver
  (CallFunction|WriteSplinePointLocations))

(event Custom|Clear%20River%20Spline
  (CallFunction|ClearWaterSpline))

(event EventBeginPlay)

(event Collision|EventActorBeginOverlap
  (params (OtherActor :type Actor%20Object%20Reference)))

(event EventTick
  (params (DeltaSeconds :type Float%20%28single-precision%29)))

(fn ConstructionScript
  (Components|StaticMesh|SetStaticMesh (Variables|Default|GetGeneratedStaticMesh) (Variables|Default|GetMesh)))

(fn WriteSplinePointLocations
  (bind _returnvalue (Actor|GetComponentbyClass "/Script/Engine.SplineComponent"))
  (bind _returnvalue_2 (Actor|GetComponentbyClass "/Script/Engine.SplineComponent"))
  (bind _returnvalue_3 (Spline|GetNumberOfSplinePoints _returnvalue_2))
  (bind _returnvalue_4 (- _returnvalue_3 1))
  (for _index (range 0 _returnvalue_4)
    (Utilities|Array|Add (Variables|Default|GetSplinePointsArray) (Spline|GetLocationatSplinePoint _returnvalue_2 _index "Local")))
  (Spline|ClearSplinePoints _returnvalue true)
  (for _index_2 (range 0 _returnvalue_4)
    (Spline|AddSplinePoint _returnvalue (Utilities|Array|Get(acopy) (Variables|Default|GetSplinePointsArray) _index_2) "Local" true))
  (Transformation|SetActorLocation "0.010000,0.000000,0.000000" false false)
  (Transformation|SetActorLocation "0, 0, 0" false false))

(fn ClearWaterSpline
  (Spline|ClearSplinePoints (Actor|GetComponentbyClass "/Script/Engine.SplineComponent") true))