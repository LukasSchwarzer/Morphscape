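; Procedural terrain actor that drives a PCG component and can shape a Water Body River from its own spline.
; BeginPlay and GeneratePCG flush the PCG cache, clean up and regenerate, with delays between steps.
; RegenTerrain also runs GenerateTerrain, defined outside these graphs, before regenerating PCG.
; Helper functions clear the river spline or copy local spline points onto it, then slightly nudge the first point.
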(event Custom|RegenTerrain
  (bind _pcg (Variables|Default|GetPCG))
  (Class|PCGBlueprintHelpers|FlushPCGCache)
  (Class|PCGComponent|Cleanup _pcg true false)
  (Utilities|FlowControl|Delay 1.0)
  (Class|ProceduralTerrain|GenerateTerrain)
  (Utilities|FlowControl|Delay 1.0)
  (PCG|Generate _pcg false))

(event Custom|Generate%20PCG
  (bind _pcg (Variables|Default|GetPCG))
  (Class|PCGBlueprintHelpers|FlushPCGCache)
  (Class|PCGComponent|Cleanup _pcg true false)
  (Utilities|FlowControl|Delay 1.0)
  (PCG|Generate _pcg false))

(event EventBeginPlay
  (bind _pcg (Variables|Default|GetPCG))
  (Utilities|FlowControl|Delay 1.0)
  (Class|PCGBlueprintHelpers|FlushPCGCache)
  (Class|PCGComponent|Cleanup _pcg true false)
  (PCG|Generate _pcg false))

(event Collision|EventActorBeginOverlap
  (params (OtherActor :type Actor%20Object%20Reference)))

(event EventTick
  (params (DeltaSeconds :type Float%20%28single-precision%29)))

(fn ConstructionScript)

(fn AssignSplinePointLocationstoRiver
  (bind _returnvalue (Actor|GetComponentbyClass "/Script/Engine.SplineComponent"))
  (bind _waterbodyriverclass (Variables|Default|GetWaterBodyRiverClass))
  (bind _splinepointsarray (Variables|Default|GetSplinePointsArray))
  (bind _returnvalue_2 (Spline|GetNumberOfSplinePoints _returnvalue))
  (bind _returnvalue_3 (Actor|GetComponentbyClass _waterbodyriverclass "/Script/Engine.SplineComponent"))
  (bind _returnvalue_4 (- _returnvalue_2 1))
  (for _index (range 0 _returnvalue_4)
    (Utilities|Array|Add (Variables|Default|GetSplinePointsArray) (Spline|GetLocationatSplinePoint _returnvalue _index "Local")))
  (Spline|ClearSplinePoints _returnvalue_3 true)
  (for _index_2 (range 0 _returnvalue_4)
    (Spline|AddSplinePoint _returnvalue_3 (Utilities|Array|Get(acopy) _splinepointsarray _index_2) "Local" true))
  (Spline|SetLocationatSplinePoint _returnvalue_3 0 (+ (Utilities|Array|Get(acopy) _splinepointsarray) "0.100000,0.000000,0.000000") "Local" true)
  (Development|PrintString "SplinePointFunctionComplete"))

(fn ClearRiverSplines
  (Spline|ClearSplinePoints (Actor|GetComponentbyClass (Variables|Default|GetWaterBodyRiverClass) "/Script/Engine.SplineComponent") true))